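; External camera Blueprint that follows a VR tracked device.
; Each tick it queries the position and orientation of the device at DeviceIndex and, when the query succeeds, passes them to UpdateOffset as the new position and rotation offsets.
; Number keys 1 to 8 switch which device index drives the offset at runtime.
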(event `Key|One`
  (params (Key :type "Key Structure"))
  ;[1 1 1] Device Index Modify by Keyboard
  (:`Pressed`
    (set `self.DeviceIndex` 1)))

(event `Key|Two`
  (params (Key :type "Key Structure"))
  ;[1 1 1] Device Index Modify by Keyboard
  (:`Pressed`
    (set `self.DeviceIndex` 2)))

(event `Key|Three`
  (params (Key :type "Key Structure"))
  ;[1 1 1] Device Index Modify by Keyboard
  (:`Pressed`
    (set `self.DeviceIndex` 3)))

(event `Key|Four`
  (params (Key :type "Key Structure"))
  ;[1 1 1] Device Index Modify by Keyboard
  (:`Pressed`
    (set `self.DeviceIndex` 4)))

(event `self.ReceiveTick`
  (params (DeltaSeconds :type "Float (single-precision)"))
  (bind (_outposition _outorientation _returnvalue) (`SteamVRFunctionLibrary.GetTrackedDevicePositionAndOrientation` (`self.DeviceIndex`)))
  ;[1 1 1] Update Offset Based on Tracking Device
  (if _returnvalue
    (`self.UpdateOffset` _outposition _outorientation)))

(event `Key|Five`
  (params (Key :type "Key Structure"))
  ;[1 1 1] Device Index Modify by Keyboard
  (:`Pressed`
    (set `self.DeviceIndex` 5)))

(event `Key|Six`
  (params (Key :type "Key Structure"))
  ;[1 1 1] Device Index Modify by Keyboard
  (:`Pressed`
    (set `self.DeviceIndex` 6)))

(event `Key|Seven`
  (params (Key :type "Key Structure"))
  ;[1 1 1] Device Index Modify by Keyboard
  (:`Pressed`
    (set `self.DeviceIndex` 7)))

(event `Key|Eight`
  (params (Key :type "Key Structure"))
  ;[1 1 1] Device Index Modify by Keyboard
  (:`Pressed`
    (set `self.DeviceIndex` 8)))

(fn `UserConstructionScript`)